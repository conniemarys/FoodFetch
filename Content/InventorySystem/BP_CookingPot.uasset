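; Cooking pot interactable that opens as a container for the player; the file contains no cooking logic.
; On interact, it casts player controller 0 to BP_PlayerController and has the HUD show the container using its inventory component.
; When looked at, it enables custom depth on the pot mesh and returns an empty string, while GetPrompt supplies the "Add to Pot" text.
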(event EventBeginPlay)

(event Collision|EventActorBeginOverlap
  (params (OtherActor :type Actor%20Object%20Reference)))

(event EventTick
  (params (DeltaSeconds :type Float%20%28single-precision%29)))

(event EventInteractwith
  (params (PlayerCharacter :type BP%20Third%20Person%20Character%20Object%20Reference))
  (bind _asbp_player_controller (Utilities|Casting|CastToBP_PlayerController (Game|GetPlayerController 0)))
  (Default|ShowContainer (Variables|/Game/ThirdPerson/Blueprints/BP_PlayerController.BP_PlayerController_C|GetHUD _asbp_player_controller) (Variables|Default|GetI_InventoryComponent)))

(fn ConstructionScript)

(fn GetPrompt
  (return "Add to Pot"))

(fn Lookat
  (Rendering|SetRenderCustomDepth (Variables|Default|GetMESH_CookingPot) true)
  (return ""))
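; Actor component that makes its owning actor a replicated inventory pickup identified by an item ID and quantity.
; On interaction it adds the stack to the player's inventory, playing a pickup effect and destroying the owner if any units fit.
; Leftover units respawn individually from the item data table's class at player 0's drop location.
; A partial or failed pickup shows a brief inventory-full widget.
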(event EventBeginPlay
  (Networking|SetReplicates (Components|GetOwner) true))

(event EventInteractwith
  (params (PlayerCharacter :type BP%20Third%20Person%20Character%20Object%20Reference))
  (bind _returnvalue (Components|GetOwner))
  (bind _returnvalue_2 (Components|GetOwner))
  (bind _inventorycomponent (Variables|/Game/ThirdPerson/Blueprints/BP_ThirdPersonCharacter.BP_ThirdPersonCharacter_C|GetInventoryComponent PlayerCharacter))
  (Utilities|IsValid _inventorycomponent
    (:Is%20Valid
      (bind _quantityremaining (Default|AddtoInventory _inventorycomponent (.rowname (Variables|Default|GetItemID)) (Variables|Default|GetQuantity)))
      ;[1 1 1] Check to see whether there was space for all items in inventory
      (Variables|Default|SetQuantity%20Remaining _quantityremaining)
      (if (== _quantityremaining 0)
        ;[1 1 1] If there is space, interact and destory actor
        (Class|IInteractInterface|Interactwith(Message) _returnvalue_2)
        (Effects|SpawnEmitteratLocation "/Game/Materials/P_PickUp.P_PickUp" (Transformation|GetActorLocation _returnvalue_2))
        (Actor|DestroyActor _returnvalue_2)
        (else
          ;[1 1 1 1 12] Comparison to see if ANY of the attempted quantity of items had space to be added
          (if (!= (Variables|Default|GetQuantity) (Variables|Default|GetQuantity%20Remaining))
            ;[1 1 1 1 12] If some, but not all, were added, destroy original actor and spawn individual units for the remaining quantity
            (Class|IInteractInterface|Interactwith(Message) _returnvalue)
            (Effects|SpawnEmitteratLocation "/Game/Materials/P_PickUp.P_PickUp" (Transformation|GetActorLocation _returnvalue))
            (Actor|DestroyActor _returnvalue)
            (bind _returnvalue_3 (Utilities|GetDataTableRow "/Game/InventorySystem/DT_ItemDataTable.DT_ItemDataTable" (.rowname (Variables|Default|GetItemID)))
              (:then
                (for _index (range 0 (- (Variables|Default|GetQuantity%20Remaining) 1))
                  ;[1 1 1 1 12] (Spawning the remaining quantity
                  (Game|SpawnActorfromClass (.itemclass _returnvalue_3) (Math|Conversions|ToTransform(Vector) (Default|GetDropLocation (Actor|GetComponentbyClass (Game|GetPlayerCharacter 0) "/Game/InventorySystem/I_InventoryComponent.I_InventoryComponent_C"))) "Undefined" 0 0)))))
          ;[1 1 1 1 10] Display 'Inventory Full' Message for 1 second
          (bind _returnvalue_4 (UserInterface|CreateWidget "/Game/InventorySystem/UI/W_InventoryFull.W_InventoryFull_C"))
          (UserInterface|Viewport|AddtoViewport _returnvalue_4 0)
          (Utilities|FlowControl|Delay 1.0)
          (Widget|RemovefromParent _returnvalue_4))))))

(fn GetUIPrompt
  (return ""))

(fn Lookat
  (return ""))
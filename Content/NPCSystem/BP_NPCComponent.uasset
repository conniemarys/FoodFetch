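; NPC component for a shop queue that handles colour choice, spawning and queue destinations for NPC1 characters.
; On BeginPlay it advances Index, wrapping at the owner's Colours count, and applies that material.
; SpawnNPC spawns an NPC1 at a fixed transform, but its queue-joining logic is unreachable.
; GetDestination returns the BP_ShopTable location for an empty queue, otherwise a point offset from the last queued NPC, mostly along world X.
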(event EventBeginPlay
  (bind _asnpc1 (Utilities|Casting|CastToNPC1 (Components|GetOwner)))
  (if (== (Utilities|Array|Length (Variables|/Game/NPCSystem/NPC1.NPC1_C|GetColours _asnpc1)) (+ (Variables|Default|GetIndex) 1))
    (Variables|Default|SetIndex 0)
    (else
      (Variables|Default|SetIndex (+ (Variables|Default|GetIndex) 1))))
  (bind _asnpc1_2 (Utilities|Casting|CastToNPC1 (Components|GetOwner)))
  (Default|ChangeMaterial _asnpc1_2 (Variables|Default|GetIndex)))

(fn SpawnNPC
  (Game|SpawnActorfromClass "/Game/NPCSystem/NPC1.NPC1_C" (Math|Transform|MakeTransform "2855.535588,-197.010140,0.000000" "0.000000,180.000000,0.000000" "1.000000,1.000000,1.000000") "Undefined" 0 0))

(fn GetDestination
  (bind _npcqueue (Variables|Default|GetNPCQueue))
  (bind _npcqueue_2 (Variables|Default|GetNPCQueue))
  (bind _returnvalue (Utilities|Array|Length _npcqueue))
  (bind _returnvalue_2 (- _returnvalue 1))
  (bind _output (Utilities|Array|Get(acopy) _npcqueue_2 _returnvalue_2))
  (bind _returnvalue_3 (Transformation|GetActorForwardVector _output))
  (if (== _returnvalue 0)
    (bind _returnvalue_4 (Actor|GetActorOfClass "/Game/CookingSystem/BP_ShopTable.BP_ShopTable_C"))
    (return (Transformation|GetActorLocation _returnvalue_4))
    (else
      (return (+ (Transformation|GetActorLocation _output) (* (Math|Vector|MakeVector (+ (.x _returnvalue_3) 1.8e+02) (.y _returnvalue_3) (.z _returnvalue_3)) "10.000000,10.000000,10.000000"))))))
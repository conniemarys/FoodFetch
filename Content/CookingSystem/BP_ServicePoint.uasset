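; Service point for a cooking system that holds a queue of recipe orders and accepts matching dishes dropped from an inventory.
; On BeginPlay it queues five random recipes from DT_RecipeDataTable, and ShowQueueUI displays them in a W_ServicePoint widget.
; A dropped dish is looked up by item ID; if ordered, the first ItemClass match is removed by manually shifting later orders down.
; The dish then leaves the inventory and the queue display refreshes.
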(event Custom|SERVER_DishDropped
  (params (InventoryComponent :type I%20Inventory%20Component%20Object%20Reference) (Index :type Integer))
  (bind _success_ (CallFunction|DishDropped InventoryComponent Index))
  (if _success_
    (Default|RemovefromInventory InventoryComponent Index false false false)
    (CallFunction|SERVERRefreshUIQueue)))

(event Custom|SERVER_RefreshUIQueue
  (Default|DisplayQueue (Variables|/Game/CookingSystem/UI/W_ServicePoint.W_ServicePoint_C|GetW_CookingQueue (Variables|Default|GetServicePointUI)) (Variables|Default|GetOrderQueue)))

(event EventBeginPlay
  (CallFunction|AddtoQueue)
  (CallFunction|AddtoQueue)
  (CallFunction|AddtoQueue)
  (CallFunction|AddtoQueue)
  (CallFunction|AddtoQueue))

(event EventTick
  (params (DeltaSeconds :type Float%20%28single-precision%29)))

(fn AddtoQueue
  (bind _outrownames (DataTable|GetDataTableRowNames "/Game/CookingSystem/DT_RecipeDataTable.DT_RecipeDataTable"))
  (bind _returnvalue (Utilities|GetDataTableRow "/Game/CookingSystem/DT_RecipeDataTable.DT_RecipeDataTable" (Utilities|Array|Get(acopy) _outrownames (Math|Random|RandomIntegerinRange 0 (- (Utilities|Array|Length _outrownames) 1))))
    (:then
      (Utilities|Array|Add (Variables|Default|GetOrderQueue) _returnvalue))))

(fn ShowQueueUI
  (bind _returnvalue (UserInterface|CreateWidget "/Game/CookingSystem/UI/W_ServicePoint.W_ServicePoint_C"))
  (Variables|Default|SetServicePointUI _returnvalue)
  (Default|DisplayQueue (Variables|/Game/CookingSystem/UI/W_ServicePoint.W_ServicePoint_C|GetW_CookingQueue _returnvalue) (Variables|Default|GetOrderQueue))
  (UserInterface|Viewport|AddtoViewport (Variables|Default|GetServicePointUI) 0))

(fn DishDropped
  (params (InventoryComponent :type I%20Inventory%20Component%20Object%20Reference) (Index :type Integer))
  (bind _returnvalue (Utilities|GetDataTableRow "/Game/CookingSystem/DT_RecipeDataTable.DT_RecipeDataTable" (.itemid (Utilities|Array|Get(acopy) (Variables|/Game/InventorySystem/I_InventoryComponent.I_InventoryComponent_C|GetContentArray InventoryComponent) Index)))
    (:then
      (bind _output_get (LocalVariables|SetRecipeToRemove _returnvalue))
      (if (Utilities|Array|ContainsItem (Variables|Default|GetOrderQueue) _output_get)
        (bind _success_ (CallFunction|RemovefromQueue (LocalVariables|GetRecipeToRemove)))
        (return _success_)
        (else
          (return false))))
    (:RowNotFound
      (return false))))

(fn RemovefromQueue
  (params (RecipeToRemove :type F%20Recipe%20Struct%20Structure))
  (LocalVariables|SetRemoved? false)
  (for _index (range 0 (- (Utilities|Array|Length (Variables|Default|GetOrderQueue)) 1))
    (LocalVariables|SetIndex _index)
    (if (LocalVariables|GetRemoved?)
      (CallFunction|RemoveRemoveOtherIndices (LocalVariables|GetIndex))
      (else
        (bind _removed_ (CallFunction|RemoveFindandRemove (LocalVariables|GetIndex) RecipeToRemove))
        (LocalVariables|SetRemoved? _removed_))))
  (if (LocalVariables|GetRemoved?)
    (return true)
    (else
      (return false))))

(fn RemoveRemoveOtherIndices
  (params (Index :type Integer))
  (bind _orderqueue (Variables|Default|GetOrderQueue))
  (if (== (+ Index 1) (Utilities|Array|Length (Variables|Default|GetOrderQueue)))
    (Utilities|Array|RemoveIndex (Variables|Default|GetOrderQueue) Index)
    (else
      (Utilities|Array|SetArrayElem _orderqueue Index (Utilities|Array|Get(acopy) _orderqueue (+ Index 1)))))
  (return))

(fn RemoveFindandRemove
  (params (Index :type Integer) (RecipeToRemove :type F%20Recipe%20Struct%20Structure))
  (bind _orderqueue (Variables|Default|GetOrderQueue))
  (if (== (.itemclass (Utilities|Array|Get(acopy) (Variables|Default|GetOrderQueue) Index)) (.itemclass RecipeToRemove))
    (if (== (Utilities|Array|Length (Variables|Default|GetOrderQueue)) (+ Index 1))
      (Utilities|Array|RemoveIndex (Variables|Default|GetOrderQueue) Index)
      (else
        (Utilities|Array|SetArrayElem _orderqueue Index (Utilities|Array|Get(acopy) _orderqueue (+ Index 1)))))
    (return true)
    (else
      (return false))))
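; Cooking component that turns the contents of its owner's inventory into a crafted item.
; On the Cook input or debug key, it sorts the inventory and seeks a DT_RecipeDataTable row whose ingredient IDs and quantities match exactly.
; A match adds the item, named by its row, to the player's inventory, then empties the owner's inventory if that succeeds.
; A W_RecipeCompleted widget then announces the recipe.
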(event Custom|Cook
  (Default|SortInventory (Variables|Default|GetInventoryComponent))
  (bind _item (CallFunction|FindRecipe))
  (if (!= _item "")
    (CallFunction|WidgetCreation _item)))

(event EventBeginPlay
  (Variables|Default|SetInventoryComponent (Actor|GetComponentbyClass (Components|GetOwner) "/Game/InventorySystem/I_InventoryComponent.I_InventoryComponent_C")))

(event EventTick
  (params (DeltaSeconds :type Float%20%28single-precision%29)))

(event Input|ActionEvents|InputActionCook
  (params (Key :type Key%20Structure))
  (:Pressed
    (CallFunction|Cook)))

(event Input|KeyboardEvents|2
  (params (Key :type Key%20Structure))
  (:Pressed
    (CallFunction|Cook)))

(fn SpawnMulch)

(fn FindRecipe
  (bind _returnvalue (Game|GetPlayerCharacter 0))
  (bind _returnvalue_2 (Actor|GetComponentbyClass _returnvalue "/Game/InventorySystem/I_InventoryComponent.I_InventoryComponent_C"))
  (LocalVariables|SetItemToSpawn "None")
  (LocalVariables|SetInventoryContents (Variables|/Game/InventorySystem/I_InventoryComponent.I_InventoryComponent_C|GetContentArray (Variables|Default|GetInventoryComponent)))
  (bind _outrownames (DataTable|GetDataTableRowNames "/Game/CookingSystem/DT_RecipeDataTable.DT_RecipeDataTable"))
  (bind _array_element (Utilities|Array|ForEachLoopwithBreak _outrownames :!label _label)
    (:LoopBody
      (bind _returnvalue_3 (Utilities|GetDataTableRow "/Game/CookingSystem/DT_RecipeDataTable.DT_RecipeDataTable" _array_element)
        (:then
          (bind _success_ (CallFunction|CompareInventories (.recipeingredients _returnvalue_3) (LocalVariables|GetInventoryContents)))
          (if _success_
            (bind _output_get (LocalVariables|SetItemToSpawn _array_element))
            (Development|PrintString (Utilities|String|ToString(Name) _output_get))
            (goto _label Break)))))
    (:Completed
      (if (!= (LocalVariables|GetItemToSpawn) "")
        (bind _success (Default|AddtoInventory _returnvalue_2 (LocalVariables|GetItemToSpawn) 1))
        (if _success
          (Default|MCUpdate _returnvalue_2)
          (for _index (range 0 (- (Utilities|Array|Length (Variables|/Game/InventorySystem/I_InventoryComponent.I_InventoryComponent_C|GetContentArray (Variables|Default|GetInventoryComponent))) 1))
            (Default|ServerRemove (Variables|Default|GetInventoryComponent) _index true false false))
          (Default|MCUpdate (Variables|Default|GetInventoryComponent))
          (return (LocalVariables|GetItemToSpawn))
          (else
            (return "None")))
        (else
          (return "None"))))))

(fn CompareInventories
  (params (RecipeComponents :type Array%20of%20F%20Slot%20Struct%20Structures) (InventoryContents :type Array%20of%20F%20Slot%20Struct%20Structures))
  (LocalVariables|SetCount 0)
  (LocalVariables|SetBreak? false)
  (CallFunction|SplitArrays RecipeComponents)
  (bind _array_element (Utilities|Array|ForEachLoopwithBreak InventoryContents :!label _label)
    (:LoopBody
      (if (!= (.itemid _array_element) "")
        (if (Utilities|Array|ContainsItem (Variables|Default|GetRecipeItemIDArray) (.itemid _array_element))
          (if (== (Utilities|Array|Get(acopy) (Variables|Default|GetRecipeQuantityArray) (Utilities|Array|FindItem (Variables|Default|GetRecipeItemIDArray) (.itemid _array_element))) (.quantity _array_element))
            (LocalVariables|SetCount (+ (LocalVariables|GetCount) (.quantity _array_element)))
            (else
              (LocalVariables|SetBreak? true :!label _label_2)
              (goto _label Break)))
          (else
            (goto _label_2)))))
    (:Completed
      (if (and (== (Variables|Default|GetRecipeTotalQuantity) (LocalVariables|GetCount)) (not (LocalVariables|GetBreak?)))
        (return true)
        (else
          (return false))))))

(fn SplitArrays
  (params (Array :type Array%20of%20F%20Slot%20Struct%20Structures))
  (for (_array_element _array_index) Array
    (if (== _array_index 0)
      (Variables|Default|SetRecipeItemIDArray (Utilities|Array|MakeArray (.itemid _array_element)))
      (Variables|Default|SetRecipeQuantityArray (Utilities|Array|MakeArray (.quantity _array_element)))
      (Variables|Default|SetRecipeTotalQuantity (.quantity _array_element))
      (else
        (Utilities|Array|Add (Variables|Default|GetRecipeItemIDArray) (.itemid _array_element))
        (Utilities|Array|Add (Variables|Default|GetRecipeQuantityArray) (.quantity _array_element))
        (Variables|Default|SetRecipeTotalQuantity (+ (Variables|Default|GetRecipeTotalQuantity) (.quantity _array_element))))))
  (return))

(fn WidgetCreation
  (params (Item :type Name))
  (bind _returnvalue (UserInterface|CreateWidget "/Game/CookingSystem/UI/W_RecipeCompleted.W_RecipeCompleted_C"))
  (bind _returnvalue_2 (Utilities|GetDataTableRow "/Game/CookingSystem/DT_RecipeDataTable.DT_RecipeDataTable" Item)
    (:then
      (Default|ChangeWidget _returnvalue (Utilities|Text|FormatText "You made {recipe}!" (.displayname _returnvalue_2)) (.thumbnail _returnvalue_2))
      (UserInterface|Viewport|AddtoViewport _returnvalue 0))))